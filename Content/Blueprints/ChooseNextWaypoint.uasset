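; Behavior tree task that picks the next patrol waypoint for an AI-controlled ThirdPersonCharacter.
; On execute it reads the pawn's PatrolPoints array, writes the entry at the blackboard Index to the Waypoint key, then finishes successfully.
; It advances Index by one with modulo on the array length, so the patrol loops back to the first point.
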(event `self.ReceiveExecuteAI`
  (params (OwnerController :type "AIController Object Reference") (ControlledPawn :type "Pawn Object Reference"))
  ;[1 1 1] Get Patrol Points
  (`self.Get Patrol Points` ControlledPawn)
  ;[1 1 1] Set Next Waypoint
  (bind _index (`self.Set Next Waypoint`))
  ;[1 1 1] Cycle Index
  (`self.Cycle Index` _index)
  (`self.FinishExecute` true))

(fn `Cycle Index`
  (params (A :type Integer))
  (`BTFunctionLibrary.SetBlackboardValueAsInt` (`self.index`) (mod (+ A 1) (`KismetArrayLibrary.Array_Length` (`self.Patrol Points`)))))

(fn `Get Patrol Points`
  (params (Object :type "Object Object Reference"))
  (bind _asthird_person_character (cast `/Game/Blueprints/ThirdPersonCharacter` Object))
  (set `self.Patrol Points` (`/Game/Blueprints/ThirdPersonCharacter.Patrol Points` _asthird_person_character)))

(fn `Set Next Waypoint`
  (returns (index :type Integer))
  (bind _returnvalue (`BTFunctionLibrary.GetBlackboardValueAsInt` (`self.index`)))
  (`BTFunctionLibrary.SetBlackboardValueAsObject` (`self.Waypoint`) (`|GetArrayItem` (`self.Patrol Points`) _returnvalue))
  (return _returnvalue))